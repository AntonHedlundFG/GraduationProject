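; Game state for the character select menu level that creates and displays the character select widget.
; Clients build the menu on BeginPlay, while the server builds it only when SetupUI is called, through the same path.
; The widget is created for player controller ID 0, given a reference to this state, added to the viewport and then refreshed.
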(event EventBeginPlay
  (if (not (Networking|IsServer))
    (bind _returnvalue (UserInterface|CreateWidget "/Game/UI/CharacterSelect/WBP_CharacterSelectMenu.WBP_CharacterSelectMenu_C" (Class|GameplayStatics|GetPlayerControllerfromID)))
    (Class|CCharacterSelectMenuWidget|SetStateRef _returnvalue self)
    (bind _output_get (Variables|Default|SetMenuWidget _returnvalue))
    (UserInterface|Viewport|AddtoViewport _output_get 0)
    (Default|UpdateUI _returnvalue)))

(event EventSetupUI
  (if (Networking|IsServer)
    (bind _returnvalue (UserInterface|CreateWidget "/Game/UI/CharacterSelect/WBP_CharacterSelectMenu.WBP_CharacterSelectMenu_C" (Class|GameplayStatics|GetPlayerControllerfromID)))
    (Class|CCharacterSelectMenuWidget|SetStateRef _returnvalue self)
    (bind _output_get (Variables|Default|SetMenuWidget _returnvalue))
    (UserInterface|Viewport|AddtoViewport _output_get 0)
    (Default|UpdateUI _returnvalue)))

(fn ConstructionScript)