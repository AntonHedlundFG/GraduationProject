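; Player controller for testing a command-based, turn-based grid game, translating Enhanced Input into requests to the server.
; On BeginPlay the local controller adds the default mapping context.
; Movement uses the Boots slot of the first unit in the game state's turn order, Attack currently requests an undo, and End Turn requests a turn end.
; Select traces under the mouse and finalizes ability use on the hit grid tile.
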(event Input|EnhancedActionEvents|EnhancedInputActionIA_MovementAbility
  (params (ActionValue :type Boolean) (ElapsedSeconds :type Float%20%28double-precision%29) (TriggeredSeconds :type Float%20%28double-precision%29) (InputAction :type Input%20Action%20Object%20Reference :default "/Game/Input/IA_MovementAbility.IA_MovementAbility"))
  (Class|CPlayerController|ServerUseObject (Utilities|Array|Get(acopy) (Variables|/Script/TacticalRogueLite.CGameState|GetTurnOrder (.AsBP%20Game%20State (Utilities|Casting|CastToBP_GameState (Game|GetGameState))))) "EIS_Boots"))

(event Input|EnhancedActionEvents|EnhancedInputActionIA_AttackAbility
  (params (ActionValue :type Boolean) (ElapsedSeconds :type Float%20%28double-precision%29) (TriggeredSeconds :type Float%20%28double-precision%29) (InputAction :type Input%20Action%20Object%20Reference :default "/Game/Input/IA_AttackAbility.IA_AttackAbility"))
  (Class|CPlayerController|ServerTryUndo))

(event Input|EnhancedActionEvents|EnhancedInputActionIA_EndTurn
  (params (ActionValue :type Boolean) (ElapsedSeconds :type Float%20%28double-precision%29) (TriggeredSeconds :type Float%20%28double-precision%29) (InputAction :type Input%20Action%20Object%20Reference :default "/Game/Input/IA_EndTurn.IA_EndTurn"))
  (Class|CPlayerController|ServerTryEndTurn))

(event Input|EnhancedActionEvents|EnhancedInputActionIA_Select
  (params (ActionValue :type Boolean) (ElapsedSeconds :type Float%20%28double-precision%29) (TriggeredSeconds :type Float%20%28double-precision%29) (InputAction :type Input%20Action%20Object%20Reference :default "/Game/Input/IA_Select.IA_Select"))
  (bind (_worldlocation _worlddirection) (Game|Player|ConvertMouseLocationToWorldSpace))
  (bind _outhit (Collision|LineTraceByChannel _worldlocation (+ _worldlocation (* _worlddirection 1e+04)) "TraceTypeQuery1" false 0 "None"))
  (bind _ascgrid_tile (Utilities|Casting|CastToCGridTile (.hitactor _outhit)))
  (Class|CPlayerController|FinalizeAbilityUse _ascgrid_tile))

(event EventBeginPlay
  (if (Pawn|IsLocalController)
    (Input|AddMappingContext (PlayerController|LocalPlayerSubsystems|GetEnhancedInputLocalPlayerSubsystem self) "/Game/Input/IMC_Default.IMC_Default" 0 "(bIgnoreAllPressedKeysUntilRelease=True,bForceImmediately=False,bNotifyUserSettings=False)")))

(fn ConstructionScript)