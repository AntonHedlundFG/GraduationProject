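; Light slash melee spell that locks the caster in place, faces the cursor and plays a slash montage, replaying it until released.
; Spell events spawn the slash VFX (Cascade or Niagara) and, on damage, briefly enable overlaps on a scaled, forward-offset hurtbox.
; Overlapped BPI_Enemy actors take directional damage and spawn impact VFX.
; On release, the caster regains movement after a short delay and the spell actor is destroyed.
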(event OnComponentBeginOverlap(SlashHurtboxCollider)
  (params (OverlappedComponent :type Primitive%20Component%20Object%20Reference) (OtherActor :type Actor%20Object%20Reference) (OtherComp :type Primitive%20Component%20Object%20Reference) (OtherBodyIndex :type Integer) (bFromSweep :type Boolean) (SweepResult :type Hit%20Result%20Structure%20%28by%20ref%29))
  ;[0 0 0 1 45] On Collision hit - Check if it's an enemy and spawn hit effects
  (bind _asbpi_enemy (Utilities|Casting|CastToBPI_Enemy OtherActor))
  (Default|DealDamage _asbpi_enemy (Math|Vector|GetUnitDirection(Vector) (Transformation|GetActorLocation) (Transformation|GetActorLocation OtherActor)) (Variables|HurtboxSettings|GetDamage%20Intensity))
  (bind _impact_vfx_position (Default|GetImpactVFXPosition _asbpi_enemy))
  (CallFunction|SpawnImpactVFX _impact_vfx_position))

(event EventDestroyed
  ;[0 0 0 1 45] On Destroyed -
  (|CallParentFunction))

(event EventOnSpellEvent01
  ;[0.3696 0.141 1 1 45] Spell Event 01 - Spawn the slash particle effects
  (|CallParentFunction)
  (CallFunction|SpawnSlashVFX))

(event EventOnSpellEvent02
  ;[0.3696 0.141 1 1 45] Spell Event 02 - Check if the spell has not been released yet. If it hasn't, replay the attack
  (|CallParentFunction)
  (if (and (Variables|Default|GetbSpellHasStarted) (not (Variables|Default|GetbSpellHasReleased)))
    (Default|LookatCursor (Variables|Default|GetCaster%20Character))
    (Default|PlayMontage (Variables|/Game/VFXASandbox/Core/Characters/BP_VFXA_Character.BP_VFXA_Character_C|GetAnimBP (Variables|Default|GetCaster%20Character)) (Variables|SpellAnimations|GetSpell%20Montage) "Default" self)
    (else
      (Animation|Montage|MontageStop (Variables|/Game/VFXASandbox/Core/Characters/BP_VFXA_Character.BP_VFXA_Character_C|GetAnimBP (Variables|Default|GetCaster%20Character)) 0.1 (Variables|SpellAnimations|GetSpell%20Montage)))))

(event EventReleaseSpell
  ;[0 0 0 1 45] Release Spell - Let the caster move again
  (|CallParentFunction)
  (Utilities|FlowControl|Delay 1.0)
  (Default|SetCharacterMobility (Variables|Default|GetCaster%20Character) true true)
  (Actor|DestroyActor))

(event EventStartSpell
  (bind _caster_character (Variables|Default|GetCaster%20Character))
  ;[0 0 0 1 45] Start Spell - Make caster immobile
  (|CallParentFunction)
  (Default|PlayMontage (Variables|/Game/VFXASandbox/Core/Characters/BP_VFXA_Character.BP_VFXA_Character_C|GetAnimBP (Variables|Default|GetCaster%20Character)) (Variables|SpellAnimations|GetSpell%20Montage) "Default" self)
  (Default|SetCharacterMobility (Variables|Default|GetCaster%20Character) false false)
  (Default|LookatCursor (Variables|Default|GetCaster%20Character))
  (Transformation|SetActorLocationAndRotation (Transformation|GetActorLocation _caster_character) (Transformation|GetActorRotation _caster_character)))

(event EventOnSpellDamage
  ;[1 0 0.0378 1 45] On Spell Damage - Activate the Hurtbox
  (|CallParentFunction)
  (CallFunction|SetupHurtbox (Variables|HurtboxSettings|GetHurtbox%20Range) (Variables|HurtboxSettings|GetHurtbox%20Width) (Variables|HurtboxSettings|GetHurtbox%20Height))
  (Variables|/Script/Engine.PrimitiveComponent|SetbGenerateOverlapEvents (Variables|Default|GetSlash%20Hurtbox%20Collider) true)
  (Utilities|FlowControl|Delay (Variables|HurtboxSettings|GetHurtbox%20Lifetime))
  (Variables|/Script/Engine.PrimitiveComponent|SetbGenerateOverlapEvents (Variables|Default|GetSlash%20Hurtbox%20Collider) false))

(fn ConstructionScript)

(fn SpawnSlashVFX
  (bind _slash_vfx (Variables|SpellVFX|GetSlash%20VFX))
  (bind _caster_character (Variables|Default|GetCaster%20Character))
  (bind _charactermovement (Variables|/Script/Engine.Character|GetCharacterMovement _caster_character))
  (bind _returnvalue (Class|CharacterMovementComponent|GetLastUpdateRotation _charactermovement))
  (bind _returnvalue_2 (Math|Rotator|CombineRotators _returnvalue "0,90.000000, 0"))
  (bind _asparticle_system (Utilities|Casting|CastToParticleSystem _slash_vfx)
    (:then
      (Effects|SpawnEmitterAttached _asparticle_system (Variables|Default|GetDefaultSceneRoot) "" (Transformation|GetActorLocation) _returnvalue_2 "1.000000,1.000000,1.000000" "KeepWorldPosition"))
    (:CastFailed
      (Niagara|SpawnSystemAttached (.AsNiagara%20System (Utilities|Casting|CastToNiagaraSystem _slash_vfx)) (Variables|Default|GetDefaultSceneRoot) "None" (Transformation|GetActorLocation) _returnvalue_2 "KeepWorldPosition" false)))
  (return))

(fn SpawnImpactVFX
  (params (Location :type Vector))
  (bind _asparticle_system (Utilities|Casting|CastToParticleSystem (Variables|SpellVFX|GetImpact%20VFX))
    (:then
      (Effects|SpawnEmitteratLocation _asparticle_system Location))
    (:CastFailed
      (Niagara|SpawnSystematLocation (.AsNiagara%20System (Utilities|Casting|CastToNiagaraSystem (Variables|SpellVFX|GetImpact%20VFX))) Location))))

(fn SetupHurtbox
  (params (Forward%20Range :type Float%20%28double-precision%29) (Width :type Float%20%28double-precision%29) (Height :type Float%20%28double-precision%29))
  (Transformation|SetRelativeScale3D (Variables|Default|GetSlash%20Hurtbox%20Collider) (Math|Vector|MakeVector Forward%20Range Width Height))
  (Transformation|SetRelativeLocation (Variables|Default|GetSlash%20Hurtbox%20Collider) (Math|Vector|MakeVector (/ Forward%20Range 1.5) 0.0 0.0) false false))