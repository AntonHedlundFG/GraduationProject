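; BP_RootAura_NiagaraActor is a visualization actor, named for a root aura Niagara effect, that follows its owner.
; Each tick it copies the owner's location and rotation without sweep or teleport.
; An unconnected graph fragment would cache the owner's CMovementAction from its CActionComponent, but it never runs.
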(event EventTick
  (params (DeltaSeconds :type Float%20%28single-precision%29))
  (bind _returnvalue (Components|GetOwner))
  (Transformation|SetActorLocation (Transformation|GetActorLocation _returnvalue) false false)
  (Transformation|SetActorRotation (Transformation|GetActorRotation _returnvalue)))

(event EventBeginPlay)

(fn ConstructionScript)