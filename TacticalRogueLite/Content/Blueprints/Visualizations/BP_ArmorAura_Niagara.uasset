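; Armor aura visualization actor that follows its owning actor.
; Every tick it moves to the owner's location with a fixed upward offset and copies the owner's rotation, rather than using attachment.
; An unconnected chain that would cache the owning unit and its movement action from the action component never runs.
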(event EventTick
  (params (DeltaSeconds :type Float%20%28single-precision%29))
  (bind _returnvalue (Components|GetOwner))
  (Transformation|SetActorLocation (+ (Transformation|GetActorLocation _returnvalue) "0.000000,0.000000,75.000000") false false)
  (Transformation|SetActorRotation (Transformation|GetActorRotation _returnvalue)))

(event EventBeginPlay)

(fn ConstructionScript)