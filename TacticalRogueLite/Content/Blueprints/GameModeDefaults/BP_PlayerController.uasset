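; Player controller for turn-based grid tactics, translating input into camera control, ability use, undo and end turn.
; On local BeginPlay it adds the input mapping, caches the SPlayerPawn and creates combat log, game menu and turn order widgets.
; Camera input is forwarded to the pawn, while number keys start abilities by equipment slot.
; Cursor line casts highlight the hovered tile on Tick and finalize abilities on left click.
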(event Input|EnhancedActionEvents|EnhancedInputActionIA_Enter
  (params (ActionValue :type Boolean) (ElapsedSeconds :type Float%20%28double-precision%29) (TriggeredSeconds :type Float%20%28double-precision%29) (InputAction :type Input%20Action%20Object%20Reference :default "/Game/Input/IA_Enter.IA_Enter"))
  (Class|SPlayerPawn|FollowActiveUnit (Variables|Default|GetControlledPawn)))

(event Input|EnhancedActionEvents|EnhancedInputActionIA_WASD
  (params (ActionValue :type Vector%202D%20Structure) (ElapsedSeconds :type Float%20%28double-precision%29) (TriggeredSeconds :type Float%20%28double-precision%29) (InputAction :type Input%20Action%20Object%20Reference :default "/Game/Input/IA_WASD.IA_WASD"))
  (Class|SPlayerPawn|MoveCameraTarget (Variables|Default|GetControlledPawn) ActionValue))

(event Input|EnhancedActionEvents|EnhancedInputActionIA_LeftMouse
  (params (ActionValue :type Boolean) (ElapsedSeconds :type Float%20%28double-precision%29) (TriggeredSeconds :type Float%20%28double-precision%29) (InputAction :type Input%20Action%20Object%20Reference :default "/Game/Input/IA_LeftMouse.IA_LeftMouse"))
  (bind (_worldlocation _worlddirection) (Game|Player|ConvertMouseLocationToWorldSpace))
  ;[1 1 1] Try Finalize Ability
  (bind (_outtile _returnvalue) (Class|CPlayerController|TryLineCastforGridTile _worldlocation _worlddirection (Variables|Default|GetGridTileLineCastRange)))
  (if _returnvalue
    (Class|CPlayerController|FinalizeAbilityUse _outtile)))

(event Input|EnhancedActionEvents|EnhancedInputActionIA_4
  (params (ActionValue :type Boolean) (ElapsedSeconds :type Float%20%28double-precision%29) (TriggeredSeconds :type Float%20%28double-precision%29) (InputAction :type Input%20Action%20Object%20Reference :default "/Game/Input/IA_4.IA_4"))
  (Class|CPlayerController|InitiateAbilityUse "(TagName=\"ItemSlot.Trinket\")"))

(event Input|EnhancedActionEvents|EnhancedInputActionIA_RightMouse
  (params (ActionValue :type Boolean) (ElapsedSeconds :type Float%20%28double-precision%29) (TriggeredSeconds :type Float%20%28double-precision%29) (InputAction :type Input%20Action%20Object%20Reference :default "/Game/Input/IA_RightMouse.IA_RightMouse"))
  (bind _controlledpawn (Variables|Default|GetControlledPawn))
  (:Started
    (Variables|/Script/Angelscript.SPlayerPawn|SetbIsRotating _controlledpawn true)
    (Class|CPlayerController|CancelAbilityUse))
  (:Canceled
    (Variables|/Script/Angelscript.SPlayerPawn|SetbIsRotating _controlledpawn false :!label _label))
  (:Completed
    (goto _label)))

(event Input|EnhancedActionEvents|EnhancedInputActionIA_MiddleMouseButtonPress
  (params (ActionValue :type Boolean) (ElapsedSeconds :type Float%20%28double-precision%29) (TriggeredSeconds :type Float%20%28double-precision%29) (InputAction :type Input%20Action%20Object%20Reference :default "/Game/Input/IA_MiddleMouseButtonPress.IA_MiddleMouseButtonPress"))
  (bind _controlledpawn (Variables|Default|GetControlledPawn))
  (:Started
    (Variables|/Script/Angelscript.SPlayerPawn|SetbIsDragging _controlledpawn true))
  (:Canceled
    (Variables|/Script/Angelscript.SPlayerPawn|SetbIsDragging _controlledpawn false :!label _label))
  (:Completed
    (goto _label)))

(event Input|EnhancedActionEvents|EnhancedInputActionIA_MouseMovement
  (params (ActionValue :type Vector%202D%20Structure) (ElapsedSeconds :type Float%20%28double-precision%29) (TriggeredSeconds :type Float%20%28double-precision%29) (InputAction :type Input%20Action%20Object%20Reference :default "/Game/Input/IA_MouseMovement.IA_MouseMovement"))
  (Class|SPlayerPawn|SetMouseMovement (Variables|Default|GetControlledPawn) ActionValue))

(event Input|EnhancedActionEvents|EnhancedInputActionIA_R
  (params (ActionValue :type Boolean) (ElapsedSeconds :type Float%20%28double-precision%29) (TriggeredSeconds :type Float%20%28double-precision%29) (InputAction :type Input%20Action%20Object%20Reference :default "/Game/Input/IA_R.IA_R"))
  (:Started
    (Class|CPlayerController|UndoAbility)))

(event Input|EnhancedActionEvents|EnhancedInputActionIA_MouseWheelScroll
  (params (ActionValue :type Float%20%28double-precision%29) (ElapsedSeconds :type Float%20%28double-precision%29) (TriggeredSeconds :type Float%20%28double-precision%29) (InputAction :type Input%20Action%20Object%20Reference :default "/Game/Input/IA_MouseWheelScroll.IA_MouseWheelScroll"))
  (Class|SPlayerPawn|Zoom (Variables|Default|GetControlledPawn) ActionValue))

(event Input|EnhancedActionEvents|EnhancedInputActionIA_3
  (params (ActionValue :type Boolean) (ElapsedSeconds :type Float%20%28double-precision%29) (TriggeredSeconds :type Float%20%28double-precision%29) (InputAction :type Input%20Action%20Object%20Reference :default "/Game/Input/IA_3.IA_3"))
  (Class|CPlayerController|InitiateAbilityUse "(TagName=\"ItemSlot.Armor\")"))

(event Input|EnhancedActionEvents|EnhancedInputActionIA_2
  (params (ActionValue :type Boolean) (ElapsedSeconds :type Float%20%28double-precision%29) (TriggeredSeconds :type Float%20%28double-precision%29) (InputAction :type Input%20Action%20Object%20Reference :default "/Game/Input/IA_2.IA_2"))
  (Class|CPlayerController|InitiateAbilityUse "(TagName=\"ItemSlot.Weapon\")"))

(event Input|EnhancedActionEvents|EnhancedInputActionIA_1
  (params (ActionValue :type Boolean) (ElapsedSeconds :type Float%20%28double-precision%29) (TriggeredSeconds :type Float%20%28double-precision%29) (InputAction :type Input%20Action%20Object%20Reference :default "/Game/Input/IA_1.IA_1"))
  (Class|CPlayerController|InitiateAbilityUse "(TagName=\"ItemSlot.Boots\")"))

(event Input|EnhancedActionEvents|EnhancedInputActionIA_SpaceBar
  (params (ActionValue :type Boolean) (ElapsedSeconds :type Float%20%28double-precision%29) (TriggeredSeconds :type Float%20%28double-precision%29) (InputAction :type Input%20Action%20Object%20Reference :default "/Game/Input/IA_SpaceBar.IA_SpaceBar"))
  (Class|CPlayerController|EndTurn))

(event EventBeginPlay
  (bind _returnvalue (Game|GetPlayerController 0))
  (if (Pawn|IsLocalController)
    (Input|AddMappingContext (PlayerController|LocalPlayerSubsystems|GetEnhancedInputLocalPlayerSubsystem self) "/Game/Input/IMC_Default.IMC_Default" 0 "(bIgnoreAllPressedKeysUntilRelease=True,bForceImmediately=False,bNotifyUserSettings=False)")
    (bind _assplayer_pawn (Utilities|Casting|CastToSPlayerPawn (Pawn|GetControlledPawn)))
    (Variables|Default|SetControlledPawn _assplayer_pawn)
    ;[1 1 1] Widget Setup
    (bind _returnvalue_2 (UserInterface|CreateWidget "/Game/UI/CombatLog/CombatLogWidget.CombatLogWidget_C" _returnvalue))
    (Class|CMovableWindow|SetUp _returnvalue_2)
    (bind _output_get (Variables|Default|SetCombatLogWidget _returnvalue_2))
    (Class|SCombatLogWidget|Initialize _output_get)
    (UserInterface|Viewport|AddtoViewport _output_get 0)
    (Input|EnableInput _returnvalue)
    (bind _returnvalue_3 (UserInterface|CreateWidget "/Game/UI/GameMenu/W_GameMenuWidget.W_GameMenuWidget_C" _returnvalue))
    (Class|CResizableWindow|SetUp _returnvalue_3)
    (bind _output_get_2 (Variables|Default|SetGameMenuWidget _returnvalue_3))
    (UserInterface|Viewport|AddtoViewport _returnvalue_3 0)
    (bind _returnvalue_4 (UserInterface|CreateWidget "/Game/UI/TurnOrder/W_TurnOrderUI.W_TurnOrderUI_C" _returnvalue))
    (UserInterface|Viewport|AddtoViewport _returnvalue_4 0)))

(event EventTick
  (params (DeltaSeconds :type Float%20%28single-precision%29))
  (bind (_worldlocation _worlddirection) (Game|Player|ConvertMouseLocationToWorldSpace))
  ;[1 1 1] Try Hover Tile
  (if (not (Utilities|Operators|EqualEqual _worldlocation (Variables|Default|GetPreviousMovePosition) 0.01))
    (bind _outtile (Class|CPlayerController|TryLineCastforGridTile _worldlocation _worlddirection (Variables|Default|GetGridTileLineCastRange)))
    (CallFunction|UpdateHoveredTile _outtile)))

(event Input|KeyboardEvents|Escape
  (params (Key :type Key%20Structure :default "None"))
  (bind _gamemenuwidget (Variables|Default|GetGameMenuWidget))
  ;[1 1 1] Open/Close Widgets
  (:Pressed
    (if (Variables|/Script/TacticalRogueLite.CMovableWindow|GetbIsOpen (Variables|Default|GetGameMenuWidget))
      (Class|CMovableWindow|Close _gamemenuwidget)
      (else
        (Class|CMovableWindow|Open _gamemenuwidget)))))

(event Input|KeyboardEvents|L
  (params (Key :type Key%20Structure :default "None"))
  (bind _combatlogwidget (Variables|Default|GetCombatLogWidget))
  ;[1 1 1] Open/Close Widgets
  (:Pressed
    (if (Variables|/Script/TacticalRogueLite.CMovableWindow|GetbIsOpen (Variables|Default|GetCombatLogWidget))
      (Class|CMovableWindow|Close _combatlogwidget)
      (else
        (Class|CMovableWindow|Open _combatlogwidget)))))

(fn ConstructionScript)

(fn UpdateHoveredTile
  (params (HoveredTile :type C%20Grid%20Tile%20Object%20Reference))
  (if (Utilities|IsValid (Variables|Default|GetLastHoveredTile))
    (Class|CHighlightComponent|RemoveHighlightMode (Variables|/Script/TacticalRogueLite.CGridTile|GetHighlightComponent (Variables|Default|GetLastHoveredTile)) "ETHM_Hovered"))
  (if (Utilities|IsValid HoveredTile)
    (bind _output_get (Variables|Default|SetLastHoveredTile HoveredTile))
    (Class|CHighlightComponent|AppendHighlightMode (Variables|/Script/TacticalRogueLite.CGridTile|GetHighlightComponent _output_get) "ETHM_Hovered")))