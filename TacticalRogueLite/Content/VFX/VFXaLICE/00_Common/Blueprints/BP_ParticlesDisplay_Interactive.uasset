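; Interactive VFX display actor that plays a timed sequence of particle effects at its location when PlayKey is pressed.
; A delayed loop spawns each EmitterSpawns entry at its SpawnTime, measured from the start time.
; Holding Shift applies TimeMultiplier to both spawn timing and emitter time dilation.
; Camera-facing text shows the key and first effect name, scales via timeline on play, and toggles with T.
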(event EventTick
  (params (DeltaSeconds :type Float%20%28single-precision%29))
  (Transformation|SetWorldRotation (Variables|Default|GetDisplay%20Text) (Camera|GetCameraRotation (Variables|/Script/Engine.PlayerController|GetPlayerCameraManager (Game|GetPlayerController 0))) false false))

(event EventBeginPlay
  (Rendering|Components|TextRender|SetText (Variables|Default|GetDisplay%20Text) (Utilities|Text|ToText(String) (Utilities|String|Append "Press " (Utilities|String|ToString(Text) (Class|KismetInputLibrary|KeyGetDisplayName (Variables|Default|GetPlay%20Key) true)))))
  (Rendering|Components|TextRender|SetText (Variables|Default|GetDisplay%20Text%20Small) (Utilities|Text|ToText(String) (Utilities|GetDisplayName (.ParticleSystem (Utilities|Struct|BreakEmitter_Spawns_Data (Utilities|Array|Get(acopy) (Variables|Default|GetEmitter%20Spawns) (Variables|PlayVariables|GetCurrentEffectIndex))))))))

(event Input|KeyboardEvents|T
  (params (Key :type Key%20Structure))
  (:Pressed
    (CallFunction|ToggleText)))

(event Input|KeyboardEvents|AnyKey
  (params (Key :type Key%20Structure))
  (:Pressed
    ;[1 1 1] Time Dilation
    (if (not (Variables|PlayVariables|GetIsPlaying))
      (if (== Key (Variables|Default|GetPlay%20Key))
        (Utilities|FlowControl|Sequence
          (:then_0
            (bind _size (Timeline|Text%20Reappear PlayFromStart)
              (:Update
                (Transformation|SetWorldScale3D (Variables|Default|GetDisplay%20Text) (Math|Vector|MakeVector _size (* -1 _size) _size)))))
          (:then_1
            (if (or (Game|Player|IsInputKeyDown (Game|GetPlayerController 0) "LeftShift") (Game|Player|IsInputKeyDown (Game|GetPlayerController 0) "RightShift"))
              (Variables|PlayVariables|SetTime%20Dilation (Variables|Default|GetTime%20Multiplier))
              (else
                (Variables|PlayVariables|SetTime%20Dilation 1.0)))
            (Variables|PlayVariables|SetStartTime (Utilities|Time|GetGameTimeinSeconds))
            (if (< (Variables|PlayVariables|GetCurrentEffectIndex) (Utilities|Array|Length (Variables|Default|GetEmitter%20Spawns))) :!label _label
              (Utilities|FlowControl|Delay (- (/ (.SpawnTime (Utilities|Struct|BreakEmitter_Spawns_Data (Utilities|Array|Get(acopy) (Variables|Default|GetEmitter%20Spawns) (Variables|PlayVariables|GetCurrentEffectIndex)))) (Variables|PlayVariables|GetTime%20Dilation)) (- (Utilities|Time|GetGameTimeinSeconds) (Variables|PlayVariables|GetStartTime))))
              (bind _returnvalue (Effects|SpawnEmitteratLocation (.ParticleSystem (Utilities|Struct|BreakEmitter_Spawns_Data (Utilities|Array|Get(acopy) (Variables|Default|GetEmitter%20Spawns) (Variables|PlayVariables|GetCurrentEffectIndex)))) (Transformation|GetActorLocation)))
              (Variables|/Script/Engine.ParticleSystemComponent|SetCustomTimeDilation _returnvalue (Variables|PlayVariables|GetTime%20Dilation))
              (Math|Integer|IncrementInt (Variables|PlayVariables|GetCurrentEffectIndex)
                (:%20%20
                  (goto _label)))
              (else
                ;[1 1 1] Reset our variables
                (Variables|PlayVariables|SetCurrentEffectIndex 0)
                (Variables|PlayVariables|SetIsPlaying false)
                (Variables|PlayVariables|SetStartTime 0.0)))))))))

(fn ConstructionScript)

(fn ToggleText
  (if (Rendering|IsVisible (Variables|Default|GetDisplay%20Text))
    (Rendering|SetVisibility (Variables|Default|GetDisplay%20Text) false true)
    (else
      (Rendering|SetVisibility (Variables|Default|GetDisplay%20Text) true true))))