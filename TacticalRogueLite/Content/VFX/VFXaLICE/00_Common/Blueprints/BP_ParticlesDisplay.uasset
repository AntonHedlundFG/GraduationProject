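; Display actor for a VFX showcase that presents an assigned Niagara or Cascade effect with a floating title.
; The construction script sets height and placeholder visibility, assigns the effect (Niagara takes priority) and titles it with the asset's name.
; On Tick the title follows camera yaw and scales in or out via a timeline as the pawn crosses a fade distance.
; The T key toggles title visibility.
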(event Custom|Show%20Text
  (Variables|Default|SetbIsTextVisible true)
  (bind _size (Timeline|Show%20Text%20Timeline Play)
    (:Update
      (Transformation|SetWorldScale3D (Variables|Default|GetTitle%20Text) (Math|Vector|MakeVector _size (* -1 _size) _size)))))

(event Custom|Hide%20Text
  (Variables|Default|SetbIsTextVisible false)
  (bind _size (Timeline|Show%20Text%20Timeline Reverse)
    (:Update
      (Transformation|SetWorldScale3D (Variables|Default|GetTitle%20Text) (Math|Vector|MakeVector _size (* -1 _size) _size)))))

(event EventBeginPlay)

(event Collision|EventActorBeginOverlap
  (params (OtherActor :type Actor%20Object%20Reference)))

(event EventTick
  (params (DeltaSeconds :type Float%20%28single-precision%29))
  (bind _returnvalue (Game|GetPlayerController 0))
  (bind _floatingtextfadedistance (Variables|Default|GetFloatingTextFadeDistance))
  (bind _title_scene (Variables|Default|GetTitle%20Scene))
  (bind _returnvalue_2 (Transformation|GetWorldLocation _title_scene))
  (bind _returnvalue_3 (Pawn|GetControlledPawn _returnvalue))
  (bind _returnvalue_4 (Transformation|GetActorLocation _returnvalue_3))
  (bind _returnvalue_5 (Math|Vector|Distance(Vector) _returnvalue_4 _returnvalue_2))
  (CallFunction|UpdateTextRotation)
  (if (Variables|Default|GetbIsTextVisible)
    (if (> _returnvalue_5 _floatingtextfadedistance)
      (CallFunction|HideText))
    (elif (< _returnvalue_5 _floatingtextfadedistance)
      (CallFunction|ShowText))))

(event Input|KeyboardEvents|T
  (params (Key :type Key%20Structure))
  (:Pressed
    (CallFunction|ToggleText)))

(fn ConstructionScript
  (bind _niagara_emitter (Variables|Default|GetNiagara%20Emitter))
  (bind _cascade_emitter (Variables|Default|GetCascade%20Emitter))
  (Transformation|SetRelativeLocation (Variables|Default|GetScene) (Math|Vector|MakeVector 0.0 0.0 (+ (Variables|Default|GetSpawn%20Height) 3e+01)) false false)
  (Rendering|SetVisibility (Variables|Default|GetSphere) (Variables|Default|GetShow%20Placeholder) false)
  (Utilities|IsValid (Variables|Default|GetNiagara%20Emitter)
    (:Is%20Valid
      (Class|NiagaraComponent|SetAsset (Variables|Default|GetNiagara%20Particle%20System) _niagara_emitter true)
      (Transformation|SetWorldScale3D (Variables|Default|GetNiagara%20Particle%20System) "1.000000,1.000000,1.000000")
      (Rendering|Components|TextRender|SetText (Variables|Default|GetTitle%20Text) (Utilities|Text|ToText(String) (Utilities|GetDisplayName _niagara_emitter))))
    (:Is%20Not%20Valid
      (Utilities|IsValid _cascade_emitter
        (:Is%20Valid
          (Effects|Components|ParticleSystem|SetTemplate (Variables|Default|GetCascade%20Particle%20System) (Variables|Default|GetCascade%20Emitter))
          (Transformation|SetWorldScale3D (Variables|Default|GetCascade%20Particle%20System) "1.000000,1.000000,1.000000")
          (Rendering|Components|TextRender|SetText (Variables|Default|GetTitle%20Text) (Utilities|Text|ToText(String) (Utilities|GetDisplayName _cascade_emitter)))))))
  (Transformation|SetWorldScale3D (Variables|Default|GetTitle%20Text) "1.000000,-1.000000,1.000000"))

(fn UpdateTextRotation
  (Transformation|SetWorldRotation (Variables|Default|GetTitle%20Scene) (Math|Rotator|MakeRotator 0.0 0.0 (.Yaw (Math|Rotator|BreakRotator (Camera|GetCameraRotation (Variables|/Script/Engine.PlayerController|GetPlayerCameraManager (Game|GetPlayerController 0)))))) false false)
  (return))

(fn ToggleText
  (if (Rendering|IsVisible (Variables|Default|GetTitle%20Scene))
    (Rendering|SetVisibility (Variables|Default|GetTitle%20Scene) false true)
    (else
      (Rendering|SetVisibility (Variables|Default|GetTitle%20Scene) true true)))
  (return))